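; BP_TankameraShot runs the photo moment in the Tankamera playground, from unlocking the shot to the flash and closing dialogue.
; LightUp counts calls and, past a threshold, shows the PremiEPerScattare prompt (Italian for "press E to shoot") and enables photo-taking on BP_Lenny.
; Flash briefly unhides the Light actor, then after a pause starts the "Caring" dialogue ending on BotPlayground.
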(event Custom|LightUp
  (bind _result (Math|Integer|IncrementInt (Variables|Default|GetLightOn))
    (:%20%20
      (if (> _result 3)
        (Rendering|SetVisibility (Variables|Default|GetPremi%20E%20per%20Scattare) true false)
        (bind _returnvalue (Actor|GetActorOfClass "/Game/Blueprints/BotsMechanics/BP_Lenny.BP_Lenny_C"))
        (Variables|/Game/Blueprints/BotsMechanics/BP_Lenny.BP_Lenny_C|SetPlayground_Tankamera_TakePhoto _returnvalue true)))))

(event Custom|Flash
  (bind _light (Variables|Default|GetLight))
  (Rendering|SetActorHiddenInGame _light false)
  (Utilities|FlowControl|Delay 0.2)
  (Rendering|SetActorHiddenInGame _light true)
  (Utilities|FlowControl|Delay 2.0)
  (Default|DialogueEndingSetup (Variables|Default|GetBot%20Playground) "Caring"))

(event EventBeginPlay)

(event Collision|EventActorBeginOverlap
  (params (OtherActor :type Actor%20Object%20Reference)))

(event EventTick
  (params (DeltaSeconds :type Float%20%28single-precision%29)))

(fn ConstructionScript)