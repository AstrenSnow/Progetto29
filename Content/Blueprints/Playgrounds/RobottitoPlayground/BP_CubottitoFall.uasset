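; BP_CubottitoFall is a trigger actor in the Robottito playground that detects BP_Cubottito actors overlapping it.
; Each overlap decrements the CubottitoNumber counter on BP_Bilancia and plays a brief Niagara burst.
; When the count reaches zero, it checks whether the Bilancia's rotation is nearly level.
; After a delay, it starts BP_Robottito's "Caring" dialogue ending and animation if level, or the "Brute" ending otherwise.
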(event EventBeginPlay)

(event Collision|EventActorBeginOverlap
  (params (OtherActor :type Actor%20Object%20Reference))
  (bind _niagara (Variables|Default|GetNiagara))
  (Utilities|Casting|CastToBP_Cubottito OtherActor)
  (bind _returnvalue (Actor|GetActorOfClass "/Game/Blueprints/Playgrounds/RobottitoPlayground/BP_Bilancia.BP_Bilancia_C"))
  (bind _result (Math|Integer|DecrementInt (Variables|/Game/Blueprints/Playgrounds/RobottitoPlayground/BP_Bilancia.BP_Bilancia_C|GetCubottitoNumber _returnvalue))
    (:%20%20
      (Components|Activation|Activate _niagara false)
      (Utilities|FlowControl|Delay 1.0)
      (Components|Activation|Deactivate _niagara)
      (if (== _result 0)
        (if (Utilities|Operators|EqualEqual :A (Transformation|GetActorRotation _returnvalue) :ErrorTolerance 2.0)
          (bind _returnvalue_2 (Actor|GetActorOfClass "/Game/Blueprints/BotsMechanics/BP_Robottito.BP_Robottito_C"))
          (Utilities|FlowControl|Delay 2.0)
          (Default|DialogueEndingSetup _returnvalue_2 "Caring")
          (Default|CaringAnimIndex _returnvalue_2)
          (else
            (bind _returnvalue_3 (Actor|GetActorOfClass "/Game/Blueprints/BotsMechanics/BP_Robottito.BP_Robottito_C"))
            (Utilities|FlowControl|Delay 2.0)
            (Default|DialogueEndingSetup _returnvalue_3 "Brute")))))))

(event EventTick
  (params (DeltaSeconds :type Float%20%28single-precision%29)))

(fn ConstructionScript)