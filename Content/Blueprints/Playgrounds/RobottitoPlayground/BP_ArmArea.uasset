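; BP_ArmArea is a trigger on one arm of the BP_Bilancia balance in the Robottito playground puzzle.
; An overlapping BP_Cubottito rotates the balance left or right according to IsLeft, decrements its cube count, then after a delay turns static, non-colliding and re-materialed.
; When the count reaches zero, a near-level balance triggers BP_Robottito's "Caring" ending dialogue and animation; otherwise it triggers the "Brute" ending.
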(event EventBeginPlay)

(event Collision|EventActorBeginOverlap
  (params (OtherActor :type Actor%20Object%20Reference))
  (bind _asbp_cubottito (Utilities|Casting|CastToBP_Cubottito OtherActor))
  (bind _returnvalue (Actor|GetActorOfClass "/Game/Blueprints/Playgrounds/RobottitoPlayground/BP_Bilancia.BP_Bilancia_C"))
  (if (Variables|Default|GetIsLeft)
    (Default|RotateLeft _returnvalue)
    (else
      (Default|RotateRight _returnvalue)))
  (Math|Integer|DecrementInt (Variables|/Game/Blueprints/Playgrounds/RobottitoPlayground/BP_Bilancia.BP_Bilancia_C|GetCubottitoNumber _returnvalue)
    (:%20%20
      (Utilities|FlowControl|Delay 1.0)
      (Transformation|SetMobility (Variables|/Game/Blueprints/Playgrounds/RobottitoPlayground/BP_Cubottito.BP_Cubottito_C|GetCube _asbp_cubottito) "Static")
      (Collision|SetCollisionEnabled (Variables|/Game/Blueprints/Playgrounds/RobottitoPlayground/BP_Cubottito.BP_Cubottito_C|GetCube _asbp_cubottito) "NoCollision")
      (Rendering|Material|SetMaterial (Variables|/Game/Blueprints/Playgrounds/RobottitoPlayground/BP_Cubottito.BP_Cubottito_C|GetCube _asbp_cubottito) 0 "/Game/EnviromentModels/Fridge/Bottiglia1_Tappo7.Bottiglia1_Tappo7")
      (if (== (Variables|/Game/Blueprints/Playgrounds/RobottitoPlayground/BP_Bilancia.BP_Bilancia_C|GetCubottitoNumber _returnvalue) 0)
        (if (Utilities|Operators|EqualEqual :A (Transformation|GetActorRotation _returnvalue) :ErrorTolerance 2.0)
          (bind _returnvalue_2 (Actor|GetActorOfClass "/Game/Blueprints/BotsMechanics/BP_Robottito.BP_Robottito_C"))
          (Utilities|FlowControl|Delay 2.0)
          (Default|DialogueEndingSetup _returnvalue_2 "Caring")
          (Default|CaringAnimIndex _returnvalue_2)
          (else
            (bind _returnvalue_3 (Actor|GetActorOfClass "/Game/Blueprints/BotsMechanics/BP_Robottito.BP_Robottito_C"))
            (Utilities|FlowControl|Delay 2.0)
            (Default|DialogueEndingSetup _returnvalue_3 "Brute")))))))

(event EventTick
  (params (DeltaSeconds :type Float%20%28single-precision%29)))

(fn ConstructionScript)