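; BP_Bilancia is a balance-scale actor ("bilancia") in the Robottito playground that tilts in fixed steps.
; On BeginPlay it counts all BP_Cubottito actors in the level and stores the total in CubottitoNumber, which this graph does not use further.
; RotateLeft and RotateRight events raise or lower the actor's pitch by a fixed increment, preserving roll and yaw; nothing in this file calls them.
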(event Custom|RotateLeft
  (bind _returnvalue (Transformation|GetActorRotation))
  (Transformation|SetActorRotation (Math|Rotator|MakeRotator (.roll _returnvalue) (+ (.pitch _returnvalue) 5.0) (.yaw _returnvalue))))

(event Custom|RotateRight
  (bind _returnvalue (Transformation|GetActorRotation))
  (Transformation|SetActorRotation (Math|Rotator|MakeRotator (.roll _returnvalue) (+ (.pitch _returnvalue) -5.0) (.yaw _returnvalue))))

(event EventBeginPlay
  (bind _outactors (Actor|GetAllActorsOfClass "/Game/Blueprints/Playgrounds/RobottitoPlayground/BP_Cubottito.BP_Cubottito_C"))
  (Variables|Default|SetCubottitoNumber (Utilities|Array|Length _outactors)))

(event Collision|EventActorBeginOverlap
  (params (OtherActor :type Actor%20Object%20Reference)))

(event EventTick
  (params (DeltaSeconds :type Float%20%28single-precision%29)))

(fn ConstructionScript)