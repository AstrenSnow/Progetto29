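; Disco prop in the Walkman playground whose Mic is rotated in steps to reach either a "Brute" or "Caring" dialogue ending.
; A LennyRoomba overlapping the box shows a text prompt and toggles Lenny's force-pin flag.
; ForceRotation takes small steps and CaringRotation larger ones toward a shared yaw threshold.
; Completion removes box and prompt, bursts Niagara, updates MicActivation actors and sets the Walkman's ending.
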(event OnComponentBeginOverlap(Box)
  (params (OverlappedComponent :type Primitive%20Component%20Object%20Reference) (OtherActor :type Actor%20Object%20Reference) (OtherComp :type Primitive%20Component%20Object%20Reference) (OtherBodyIndex :type Integer) (bFromSweep :type Boolean) (SweepResult :type Hit%20Result%20Structure%20%28by%20ref%29))
  (Utilities|Casting|CastToBP_LennyRoomba OtherActor)
  (bind _returnvalue (Actor|GetActorOfClass "/Game/Blueprints/BotsMechanics/BP_Lenny.BP_Lenny_C"))
  (Variables|/Game/Blueprints/BotsMechanics/BP_Lenny.BP_Lenny_C|SetPlayground_Walkman_ForcePin _returnvalue true)
  (Rendering|SetVisibility (Variables|Default|GetTextRender) true false))

(event OnComponentEndOverlap(Box)
  (params (OverlappedComponent :type Primitive%20Component%20Object%20Reference) (OtherActor :type Actor%20Object%20Reference) (OtherComp :type Primitive%20Component%20Object%20Reference) (OtherBodyIndex :type Integer))
  (Utilities|Casting|CastToBP_LennyRoomba OtherActor)
  (bind _returnvalue (Actor|GetActorOfClass "/Game/Blueprints/BotsMechanics/BP_Lenny.BP_Lenny_C"))
  (Variables|/Game/Blueprints/BotsMechanics/BP_Lenny.BP_Lenny_C|SetPlayground_Walkman_ForcePin _returnvalue false)
  (Rendering|SetVisibility (Variables|Default|GetTextRender) false false))

(event Custom|ForceRotation
  (bind _mic (Variables|Default|GetMic))
  (bind _niagara (Variables|Default|GetNiagara))
  (bind _returnvalue (Transformation|GetWorldTransform _mic))
  (Transformation|SetWorldTransform _mic (Math|Transform|MakeTransform (.location _returnvalue) (Math|Rotator|MakeRotator (.roll (.rotation _returnvalue)) (.pitch (.rotation _returnvalue)) (+ (.yaw (.rotation _returnvalue)) 5.0)) (.scale _returnvalue)) false false)
  (bind _output_get (Variables|Default|SetChangedRotation (+ (Variables|Default|GetChangedRotation) 5.0)))
  (if (>= _output_get 4e+01)
    (bind _outactors (Actor|GetAllActorsOfClass "/Game/Blueprints/Playgrounds/WalkmanPlayground/BP_MicActivation.BP_MicActivation_C"))
    (for _array_element _outactors
      (Default|EndedPlayground _array_element))
    (Components|DestroyComponent (Variables|Default|GetBox))
    (bind _returnvalue_2 (Actor|GetActorOfClass "/Game/Blueprints/BotsMechanics/BP_Lenny.BP_Lenny_C"))
    (Variables|/Game/Blueprints/BotsMechanics/BP_Lenny.BP_Lenny_C|SetPlayground_Walkman_ForcePin _returnvalue_2 false)
    (Components|Activation|Activate _niagara false)
    (Utilities|FlowControl|Delay 1.5)
    (Components|Activation|Deactivate _niagara)
    (bind _returnvalue_3 (Actor|GetActorOfClass "/Game/Blueprints/BotsMechanics/BP_Walkman.BP_Walkman_C"))
    (Default|DialogueEndingSetup _returnvalue_3 "Brute")))

(event Custom|CaringRotation
  (bind _mic (Variables|Default|GetMic))
  (bind _niagara (Variables|Default|GetNiagara))
  (bind _returnvalue (Transformation|GetWorldTransform _mic))
  (Transformation|SetWorldTransform _mic (Math|Transform|MakeTransform (.location _returnvalue) (Math|Rotator|MakeRotator (.roll (.rotation _returnvalue)) (.pitch (.rotation _returnvalue)) (+ (.yaw (.rotation _returnvalue)) 2e+01)) (.scale _returnvalue)) false false)
  (bind _output_get (Variables|Default|SetChangedRotation (+ (Variables|Default|GetChangedRotation) 2e+01)))
  (if (>= _output_get 4e+01)
    (Components|DestroyComponent (Variables|Default|GetBox))
    (Components|Activation|Activate _niagara false)
    (Utilities|FlowControl|Delay 2.0)
    (Components|Activation|Deactivate _niagara)
    (bind _outactors (Actor|GetAllActorsOfClass "/Game/Blueprints/Playgrounds/WalkmanPlayground/BP_MicActivation.BP_MicActivation_C"))
    (for _array_element _outactors
      (Components|Activation|Deactivate (Variables|/Game/Blueprints/Playgrounds/WalkmanPlayground/BP_MicActivation.BP_MicActivation_C|GetNiagara _array_element)))
    (bind _returnvalue_2 (Actor|GetActorOfClass "/Game/Blueprints/BotsMechanics/BP_Walkman.BP_Walkman_C"))
    (Default|DialogueEndingSetup _returnvalue_2 "Caring")))

(event EventBeginPlay)

(event Collision|EventActorBeginOverlap
  (params (OtherActor :type Actor%20Object%20Reference)))

(event EventTick
  (params (DeltaSeconds :type Float%20%28single-precision%29)))

(fn ConstructionScript)