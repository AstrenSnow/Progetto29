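; Microphone activation trigger for the Walkman playground, armed while BP_LennyRoomba overlaps it.
; Overlap begin and end toggle the microphone-activation flag on BP_Lenny and the visibility of a text prompt.
; ActivateMicrophone calls CaringRotation on BP_Disco, starts a Niagara effect, clears Lenny's flag and destroys the Box and text.
; EndedPlayground destroys those same two components without activating anything.
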(event Custom|ActivateMicrophone
  (bind _returnvalue (Actor|GetActorOfClass "/Game/Blueprints/Playgrounds/WalkmanPlayground/BP_Disco.BP_Disco_C"))
  (Default|CaringRotation _returnvalue)
  (Components|Activation|Activate (Variables|Default|GetNiagara) false)
  (bind _returnvalue_2 (Actor|GetActorOfClass "/Game/Blueprints/BotsMechanics/BP_Lenny.BP_Lenny_C"))
  (Variables|/Game/Blueprints/BotsMechanics/BP_Lenny.BP_Lenny_C|SetPlayground_Walkman_ActivateMicrophone _returnvalue_2 false)
  (Components|DestroyComponent (Variables|Default|GetBox)))

(event Custom|EndedPlayground
  (Components|DestroyComponent (Variables|Default|GetBox)))

(event EventBeginPlay)

(event Collision|EventActorBeginOverlap
  (params (OtherActor :type Actor%20Object%20Reference))
  (Utilities|Casting|CastToBP_LennyRoomba OtherActor)
  (bind _returnvalue (Actor|GetActorOfClass "/Game/Blueprints/BotsMechanics/BP_Lenny.BP_Lenny_C"))
  (Variables|/Game/Blueprints/BotsMechanics/BP_Lenny.BP_Lenny_C|SetPlayground_Walkman_ActivateMicrophone _returnvalue true)
  (Rendering|SetVisibility (Variables|Default|GetTextRender) true false))

(event EventTick
  (params (DeltaSeconds :type Float%20%28single-precision%29)))

(event Collision|EventActorEndOverlap
  (params (OtherActor :type Actor%20Object%20Reference))
  (Utilities|Casting|CastToBP_LennyRoomba OtherActor)
  (bind _returnvalue (Actor|GetActorOfClass "/Game/Blueprints/BotsMechanics/BP_Lenny.BP_Lenny_C"))
  (Variables|/Game/Blueprints/BotsMechanics/BP_Lenny.BP_Lenny_C|SetPlayground_Walkman_ActivateMicrophone _returnvalue false)
  (Rendering|SetVisibility (Variables|Default|GetTextRender) false false))

(fn ConstructionScript)