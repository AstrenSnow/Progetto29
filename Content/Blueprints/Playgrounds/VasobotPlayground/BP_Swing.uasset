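; Playground swing in the Vasobot level that judges the player as brute or caring by how hard they push.
; BP_LennyRoomba overlaps toggle the prompt text, and both set Lenny's can-swing flag true.
; Charge and activate events time the press, growing a decal while held, to pick a strong or gentle roll timeline.
; After three swings, the majority type picks BP_Vasobot's Brute or Caring ending dialogue.
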(event Custom|ChargeSwing
  (Variables|Default|SetIsCharging true)
  (Variables|Default|SetPressStartTime (Utilities|Time|GetGameTimeinSeconds))
  (Rendering|SetVisibility (Variables|Default|GetTextRender) false false))

(event Custom|ActivateSwing
  (bind _swing (Variables|Default|GetSwing))
  (bind _returnvalue (Transformation|GetWorldRotation _swing))
  (bind _returnvalue_2 (Transformation|GetWorldRotation _swing))
  (Variables|Default|SetIsCharging false)
  (bind _output_get (Variables|Default|SetPressDuration (- (Utilities|Time|GetGameTimeinSeconds) (Variables|Default|GetPressStartTime))))
  (if (> _output_get 3.0)
    (bind _strongswing (Timeline|Timeline PlayFromStart)
      (:Update
        (Transformation|SetWorldRotation _swing (Math|Rotator|MakeRotator _strongswing (.pitch _returnvalue) (.yaw _returnvalue)) false false))
      (:Finished
        (bind _result (Math|Integer|IncrementInt (Variables|Default|GetTimesStrong))
          (:%20%20
            (bind _output_get_2 (Variables|Default|SetTotalSwings (+ _result (stale _result_2)) :!label _label))
            (if (>= _output_get_2 3)
              (Utilities|FlowControl|Delay 2.0)
              (if (> (Variables|Default|GetTimesStrong) (Variables|Default|GetTimesGentle))
                (bind _returnvalue_3 (Actor|GetActorOfClass "/Game/Blueprints/BotsMechanics/BP_Vasobot.BP_Vasobot_C"))
                (Default|DialogueEndingSetup _returnvalue_3 "Brute")
                (else
                  (bind _returnvalue_4 (Actor|GetActorOfClass "/Game/Blueprints/BotsMechanics/BP_Vasobot.BP_Vasobot_C"))
                  (Default|DialogueEndingSetup _returnvalue_4 "Caring")
                  (Variables|/Game/Blueprints/BotsMechanics/BP_Vasobot.BP_Vasobot_C|SetCaring _returnvalue_4 true)))
              (else
                (Rendering|SetVisibility (Variables|Default|GetTextRender) true false)
                (bind _returnvalue_5 (Actor|GetActorOfClass "/Game/Blueprints/BotsMechanics/BP_Lenny.BP_Lenny_C"))
                (Variables|/Game/Blueprints/BotsMechanics/BP_Lenny.BP_Lenny_C|SetPlayground_Vasobot_CanSwing _returnvalue_5 true)))))))
    (else
      (bind _gentleswing (Timeline|Timeline_0 PlayFromStart)
        (:Update
          (Transformation|SetWorldRotation _swing (Math|Rotator|MakeRotator _gentleswing (.pitch _returnvalue_2) (.yaw _returnvalue_2)) false false))
        (:Finished
          (bind _result_2 (Math|Integer|IncrementInt (Variables|Default|GetTimesGentle))
            (:%20%20
              (goto _label))))))))

(event EventBeginPlay)

(event Collision|EventActorBeginOverlap
  (params (OtherActor :type Actor%20Object%20Reference))
  (Utilities|Casting|CastToBP_LennyRoomba OtherActor)
  (Rendering|SetVisibility (Variables|Default|GetTextRender) true false)
  (bind _returnvalue (Actor|GetActorOfClass "/Game/Blueprints/BotsMechanics/BP_Lenny.BP_Lenny_C"))
  (Variables|/Game/Blueprints/BotsMechanics/BP_Lenny.BP_Lenny_C|SetPlayground_Vasobot_CanSwing _returnvalue true))

(event Collision|EventActorEndOverlap
  (params (OtherActor :type Actor%20Object%20Reference))
  (Utilities|Casting|CastToBP_LennyRoomba OtherActor)
  (Rendering|SetVisibility (Variables|Default|GetTextRender) false false)
  (bind _returnvalue (Actor|GetActorOfClass "/Game/Blueprints/BotsMechanics/BP_Lenny.BP_Lenny_C"))
  (Variables|/Game/Blueprints/BotsMechanics/BP_Lenny.BP_Lenny_C|SetPlayground_Vasobot_CanSwing _returnvalue true))

(event EventTick
  (params (DeltaSeconds :type Float%20%28single-precision%29))
  (bind _decal (Variables|Default|GetDecal))
  (bind _decal_2 (Variables|Default|GetDecal))
  (bind _returnvalue (Transformation|GetWorldTransform _decal_2))
  (bind _returnvalue_2 (Transformation|GetWorldTransform _decal))
  (if (Variables|Default|GetIsCharging)
    (Transformation|SetWorldTransform _decal (Math|Transform|MakeTransform (.location _returnvalue_2) (.rotation _returnvalue_2) (+ (.scale _returnvalue_2) "0.100000,0.100000,0.100000")) false false)
    (elif (not (< (.x (.scale (Transformation|GetWorldTransform _decal))) 0.0))
      (Transformation|SetWorldTransform _decal_2 (Math|Transform|MakeTransform (.location _returnvalue) (.rotation _returnvalue) (+ (.scale _returnvalue) "-0.100000,-0.100000,-0.100000")) false false))))

(fn ConstructionScript)