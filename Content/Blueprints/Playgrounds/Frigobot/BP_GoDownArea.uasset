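; BP_GoDownArea is a trigger area in the Frigobot playground that signals when the Lenny roomba can get down.
; On begin play it caches the BP_Lenny actor in the level.
; When a BP_LennyRoomba overlaps it, it shows a text prompt and sets PlaygroundFrigobotGetDown on Lenny, then hides and clears both when the overlap ends.
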(event EventBeginPlay
  (bind _returnvalue (Actor|GetActorOfClass "/Game/Blueprints/BotsMechanics/BP_Lenny.BP_Lenny_C"))
  (Variables|Default|SetCharacterRef _returnvalue))

(event Collision|EventActorBeginOverlap
  (params (OtherActor :type Actor%20Object%20Reference))
  (Utilities|Casting|CastToBP_LennyRoomba OtherActor)
  (Rendering|SetVisibility (Variables|Default|GetTextRender) true false)
  (Variables|/Game/Blueprints/BotsMechanics/BP_Lenny.BP_Lenny_C|SetPlayground_Frigobot_GetDown (Variables|Default|GetCharacterRef) true))

(event Collision|EventActorEndOverlap
  (params (OtherActor :type Actor%20Object%20Reference))
  (Utilities|Casting|CastToBP_LennyRoomba OtherActor)
  (Rendering|SetVisibility (Variables|Default|GetTextRender) false false)
  (Variables|/Game/Blueprints/BotsMechanics/BP_Lenny.BP_Lenny_C|SetPlayground_Frigobot_GetDown (Variables|Default|GetCharacterRef) false))

(fn ConstructionScript)