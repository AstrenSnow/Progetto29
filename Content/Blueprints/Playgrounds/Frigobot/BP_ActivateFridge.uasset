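; BP_ActivateFridge is an interactable fridge trigger for the Frigobot playground, tracking activations toward its ending dialogue.
; Overlap with BP_LennyRoomba toggles a text prompt; both enter and exit set BP_Lenny's activate-fridge flag to true.
; ActivateSmoke re-applies the Smoke actor's own location and rotation and increments Lenny's activation counter.
; It then destroys itself, first triggering BP_FrigoBot's "Caring" ending after a short delay once the count passes its threshold.
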(event Custom|ActivateSmoke
  (bind _smoke (Variables|Default|GetSmoke))
  (bind _returnvalue (Transformation|GetActorTransform _smoke))
  (Transformation|SetActorTransform _smoke (Math|Transform|MakeTransform (.location _returnvalue) (.rotation _returnvalue) "1.000000,1.000000,1.000000"))
  (bind _result (Math|Integer|IncrementInt (Variables|/Game/Blueprints/BotsMechanics/BP_Lenny.BP_Lenny_C|GetPlayground_Frigobot_NumberActivated (Variables|Default|GetCharacterRef)))
    (:%20%20
      (if (> _result 3)
        (Utilities|FlowControl|Delay 1.0)
        (bind _returnvalue_2 (Actor|GetActorOfClass "/Game/Blueprints/BotsMechanics/BP_FrigoBot.BP_FrigoBot_C"))
        (Default|DialogueEndingSetup _returnvalue_2 "Caring")
        (Actor|DestroyActor)
        (else
          (Actor|DestroyActor))))))

(event EventBeginPlay
  (bind _returnvalue (Actor|GetActorOfClass "/Game/Blueprints/BotsMechanics/BP_Lenny.BP_Lenny_C"))
  (Variables|Default|SetCharacterRef _returnvalue))

(event Collision|EventActorBeginOverlap
  (params (OtherActor :type Actor%20Object%20Reference))
  (Utilities|Casting|CastToBP_LennyRoomba OtherActor)
  (Rendering|SetVisibility (Variables|Default|GetTextRender) true false)
  (Variables|/Game/Blueprints/BotsMechanics/BP_Lenny.BP_Lenny_C|SetPlayground_Frigobot_ActivateFridge (Variables|Default|GetCharacterRef) true))

(event Collision|EventActorEndOverlap
  (params (OtherActor :type Actor%20Object%20Reference))
  (Utilities|Casting|CastToBP_LennyRoomba OtherActor)
  (Rendering|SetVisibility (Variables|Default|GetTextRender) false false)
  (Variables|/Game/Blueprints/BotsMechanics/BP_Lenny.BP_Lenny_C|SetPlayground_Frigobot_ActivateFridge (Variables|Default|GetCharacterRef) true))

(fn ConstructionScript)