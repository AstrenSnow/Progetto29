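; Exit zone actor in the bot playground that triggers the "Ignavo" dialogue ending when BP_LennyRoomba lingers in it.
; Entering the box sets a leaving flag and starts a four-second delay, then rechecks overlapping roombas before calling DialogueEndingSetup on BotPlayground.
; Tick grows a decal by a fixed per-frame step while the flag is set and shrinks it back toward zero scale once the roomba exits.
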(event OnComponentBeginOverlap(Box)
  (params (OverlappedComponent :type Primitive%20Component%20Object%20Reference) (OtherActor :type Actor%20Object%20Reference) (OtherComp :type Primitive%20Component%20Object%20Reference) (OtherBodyIndex :type Integer) (bFromSweep :type Boolean) (SweepResult :type Hit%20Result%20Structure%20%28by%20ref%29))
  (Utilities|Casting|CastToBP_LennyRoomba OtherActor)
  (Variables|Default|SetIsLeaving true)
  (Utilities|FlowControl|Delay 4.0)
  (for _array_element (Collision|GetOverlappingActors (Variables|Default|GetBox) "/Game/Blueprints/BotsMechanics/BP_LennyRoomba.BP_LennyRoomba_C" :!class /Script/Engine.PrimitiveComponent)
    (if (!= _array_element 0)
      (Default|DialogueEndingSetup (Variables|Default|GetBotPlayground) "Ignavo")
      (else
        (Variables|Default|SetIsLeaving false)))))

(event OnComponentEndOverlap(Box)
  (params (OverlappedComponent :type Primitive%20Component%20Object%20Reference) (OtherActor :type Actor%20Object%20Reference) (OtherComp :type Primitive%20Component%20Object%20Reference) (OtherBodyIndex :type Integer))
  (Utilities|Casting|CastToBP_LennyRoomba OtherActor)
  (Variables|Default|SetIsLeaving false))

(event EventBeginPlay)

(event Collision|EventActorBeginOverlap
  (params (OtherActor :type Actor%20Object%20Reference)))

(event EventTick
  (params (DeltaSeconds :type Float%20%28single-precision%29))
  (bind _decal (Variables|Default|GetDecal))
  (bind _decalchange (Variables|Default|GetDecalChange))
  (bind _returnvalue (Transformation|GetWorldTransform _decal))
  (if (Variables|Default|GetIsLeaving)
    (Transformation|SetWorldTransform _decal (Math|Transform|MakeTransform (.location _returnvalue) (.rotation _returnvalue) (+ (.scale _returnvalue) _decalchange)) false false)
    (elif (Class|KismetMathLibrary|NotEqualExactlyVectorVector (.scale _returnvalue) "0, 0, 0")
      (Transformation|SetWorldTransform _decal (Math|Transform|MakeTransform (.location _returnvalue) (.rotation _returnvalue) (- (.scale _returnvalue) _decalchange)) false false))))

(fn ConstructionScript)