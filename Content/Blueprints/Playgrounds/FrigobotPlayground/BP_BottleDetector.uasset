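; Trigger actor in the Frigobot playground that detects bottles and triggers an ending dialogue once enough have been dropped.
; At BeginPlay it counts all BP_Bottle actors in the level as the target.
; Each bottle overlap activates a Niagara effect briefly and increments a drop counter, without checking for repeat bottles.
; When the counter reaches the target, it waits, calls the playground's "Brute" ending dialogue, then deactivates the effect.
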(event EventBeginPlay
  (bind _outactors (Actor|GetAllActorsOfClass "/Game/Blueprints/Playgrounds/FrigobotPlayground/BP_Bottle.BP_Bottle_C"))
  (for _array_element _outactors
    (Math|Integer|IncrementInt (Variables|Default|GetBottleNumber))))

(event Collision|EventActorBeginOverlap
  (params (OtherActor :type Actor%20Object%20Reference))
  (bind _niagara (Variables|Default|GetNiagara))
  (Utilities|Casting|CastToBP_Bottle OtherActor)
  (Components|Activation|Activate _niagara false)
  (Math|Integer|IncrementInt (Variables|Default|GetBottleDropNumber)
    (:%20%20
      (if (>= (Variables|Default|GetBottleDropNumber) (Variables|Default|GetBottleNumber))
        (Utilities|FlowControl|Delay 2.0)
        (Default|DialogueEndingSetup (Variables|Default|GetBot_Playground) "Brute")
        (Components|Activation|Deactivate _niagara)
        (else
          (Utilities|FlowControl|Delay 0.2)
          (Components|Activation|Deactivate _niagara))))))

(event EventTick
  (params (DeltaSeconds :type Float%20%28single-precision%29)))

(fn ConstructionScript)