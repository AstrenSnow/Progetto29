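; Vasobot is a bot character that ends up on Lenny's head once its dialogue finishes.
; A looping event picks a random animation index every three seconds and resets the index on its ABP_Vasetto anim instance.
; Tick watches for the last dialogue line while Caring, then sets Jump and, once, waits briefly, hides the actor and calls VasobotOnHead on BP_Lenny.
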(event Custom|AnimIndex
  (Variables|Default|SetAnimationIndex (Math|Random|RandomInteger 2))
  (Utilities|FlowControl|Delay 3.0)
  (bind _asabp_vasetto (Utilities|Casting|CastToABP_Vasetto (Components|SkeletalMesh|GetAnimInstance (Variables|Default|GetVaso))))
  (Default|ResetIndex _asabp_vasetto)
  (CallFunction|AnimIndex))

(event EventBeginPlay
  (|CallParentFunction)
  (CallFunction|AnimIndex)
  (Variables|Default|SetUIName "Vasobot"))

(event Collision|EventActorBeginOverlap
  (params (OtherActor :type Actor%20Object%20Reference)))

(event EventTick
  (params (DeltaSeconds :type Float%20%28single-precision%29))
  (|CallParentFunction DeltaSeconds)
  (if (and (== (Variables|Default|GetDialogueIndex) (Utilities|Array|Length (Variables|Default|GetDialogueStrings))) (Variables|Default|GetCaring))
    (Variables|Default|SetJump true)
    (Utilities|FlowControl|DoOnce false
      (:Completed
        (Utilities|FlowControl|Delay 4.5)
        (Rendering|SetActorHiddenInGame true)
        (bind _returnvalue (Actor|GetActorOfClass "/Game/Blueprints/BotsMechanics/BP_Lenny.BP_Lenny_C"))
        (Default|VasobotonHead _returnvalue)))))

(fn ConstructionScript
  (|CallParentFunction))