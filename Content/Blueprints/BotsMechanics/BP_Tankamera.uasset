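; BP_Tankamera is the Blueprint for the Tankamera bot, which sets its UI name on BeginPlay and cycles its animation at random.
; A self-calling AnimIndex event picks one of three random animation indices, waits two seconds, then calls ResetIndex on the mesh's ABP_Tankamera anim instance and repeats.
; The loop stops if that anim instance cast fails.
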(event Custom|AnimIndex
  (Variables|Default|SetAnimationIndex (Math|Random|RandomInteger 3))
  (Utilities|FlowControl|Delay 2.0)
  (bind _asabp_tankamera (Utilities|Casting|CastToABP_Tankamera (Components|SkeletalMesh|GetAnimInstance (Variables|Default|GetTankamera))))
  (Default|ResetIndex _asabp_tankamera)
  (CallFunction|AnimIndex))

(event EventBeginPlay
  (|CallParentFunction)
  (CallFunction|AnimIndex)
  (Variables|Default|SetUIName "Tankamera"))

(event Collision|EventActorBeginOverlap
  (params (OtherActor :type Actor%20Object%20Reference)))

(event EventTick
  (params (DeltaSeconds :type Float%20%28single-precision%29))
  (|CallParentFunction DeltaSeconds) ; This node is disabled and will not be called.\nDrag off pins to build functionality.
)

(fn ConstructionScript
  (|CallParentFunction))