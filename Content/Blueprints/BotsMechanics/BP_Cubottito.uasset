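; BP_Cubottito is a bot Blueprint that presents itself in the UI as Robottito and relies on its parent class for most behavior.
; BeginPlay runs the parent logic, fires AnimIndex, then sets the UI name.
; AnimIndex toggles IsFlipped, then casts the Cubottito mesh's anim instance to ABP_Robottito and calls ResetIndex on it.
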(event Custom|AnimIndex
  (Variables|Default|SetIsFlipped (not (Variables|Default|GetIsFlipped)))
  (bind _asabp_robottito (Utilities|Casting|CastToABP_Robottito (Components|SkeletalMesh|GetAnimInstance (Variables|Default|GetCubottito))))
  (Default|ResetIndex _asabp_robottito))

(event EventBeginPlay
  (|CallParentFunction)
  (CallFunction|AnimIndex)
  (Variables|Default|SetUIName "Robottito"))

(event Collision|EventActorBeginOverlap
  (params (OtherActor :type Actor%20Object%20Reference)))

(event EventTick
  (params (DeltaSeconds :type Float%20%28single-precision%29))
  (|CallParentFunction DeltaSeconds) ; This node is disabled and will not be called.\nDrag off pins to build functionality.
)

(fn ConstructionScript
  (|CallParentFunction))