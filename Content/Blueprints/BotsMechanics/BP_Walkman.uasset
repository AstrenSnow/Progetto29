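; BP_Walkman is a Walkman bot Blueprint that labels itself "Walkman" for UI and periodically randomizes its animation index.
; On BeginPlay it runs parent logic and starts AnimIndex, a self-recalling event that picks one of three indices and waits three seconds.
; It then calls ResetIndex on the mesh's ABP_Walkman anim instance and repeats, stopping if that cast fails.
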(event Custom|AnimIndex
  (Variables|Default|SetAnimationIndex (Math|Random|RandomInteger 3))
  (Utilities|FlowControl|Delay 3.0)
  (bind _asabp_walkman (Utilities|Casting|CastToABP_Walkman (Components|SkeletalMesh|GetAnimInstance (Variables|Default|GetWalkman))))
  (Default|ResetIndex _asabp_walkman)
  (CallFunction|AnimIndex))

(event EventBeginPlay
  (|CallParentFunction)
  (CallFunction|AnimIndex)
  (Variables|Default|SetUIName "Walkman"))

(event Collision|EventActorBeginOverlap
  (params (OtherActor :type Actor%20Object%20Reference)))

(event EventTick
  (params (DeltaSeconds :type Float%20%28single-precision%29))
  (|CallParentFunction DeltaSeconds) ; This node is disabled and will not be called.\nDrag off pins to build functionality.
)

(fn ConstructionScript
  (|CallParentFunction))