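; Base selectable world actor that shows a floating UI, text description and decals to signal seen and selected states.
; Enable and disable events toggle the seen decal, UI and text, with enabling blocked while selected.
; Selecting or deselecting hides the hover UI and toggles the selected decal.
; Tick yaw-rotates the UI relative to the player camera with an image offset, while both state query functions always return false.
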(event EventTick
  (params (DeltaSeconds :type Float%20%28single-precision%29))
  (Transformation|SetRelativeRotation (Variables|Default|GetUI) (Math|Rotator|MakeRotator 0.0 0.0 (+ (.Yaw (Math|Rotator|BreakRotator (Math|Rotator|FindLookatRotation (Camera|GetCameraLocation (Game|GetPlayerCameraManager 0)) (Transformation|GetActorLocation)))) (Variables|Default|GetRotationFixImage))) false false))

(event EventEnableUI
  (if (not (Variables|Default|GetIsSelected))
    (Rendering|SetVisibility (Variables|Default|GetUIDecalOnSeen) true false)
    (Rendering|SetVisibility (Variables|Default|GetUI) true false)))

(event EventDisableUI
  (Rendering|SetVisibility (Variables|Default|GetUIDecalOnSeen) false false)
  (Rendering|SetVisibility (Variables|Default|GetUI) false false))

(event EventUISelected
  (Variables|Default|SetIsSelected true)
  (CallFunction|DisableUI)
  (Rendering|SetVisibility (Variables|Default|GetUIDecalOnSelected) true false))

(event EventUIDeselected
  (Variables|Default|SetIsSelected false)
  (CallFunction|DisableUI)
  (Rendering|SetVisibility (Variables|Default|GetUIDecalOnSelected) false false))

(fn ConstructionScript)

(fn IsSelected?
  (return false))

(fn UIActive?
  (return false))